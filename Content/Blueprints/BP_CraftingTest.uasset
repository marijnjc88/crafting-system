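; BP_CraftingTest is a test actor that runs the weapon crafting pipeline on BeginPlay and prints the results on screen.
; It aggregates the resources in CraftingInput, generates weapon stats for WeaponType from that aggregation, then prints damage, durability and attack speed as long-lived keyed messages.
; An unwired PrintResourceAggregation helper can also print each aggregated stat's average, highest and most influential resource.
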(event EventBeginPlay
  (bind _weapontype (Variables|Default|GetWeaponType))
  (bind _returnvalue (Class|ProceduralCraftingFunctionLibrary|AggregateResources (Variables|Default|GetCraftingInput)))
  (bind _returnvalue_2 (Class|ProceduralCraftingFunctionLibrary|GenerateWeaponStats _returnvalue _weapontype))
  (CallFunction|PrintWeaponStats _returnvalue_2 _weapontype))

(event Collision|EventActorBeginOverlap
  (params (OtherActor :type Actor%20Object%20Reference)))

(event EventTick
  (params (DeltaSeconds :type Float%20%28single-precision%29)))

(fn ConstructionScript)

(fn PrintResourceAggregation
  (params (ResourceAggregation :type Resource%20Aggregation%20Structure%20%28by%20ref%29))
  (bind _valuepin (Utilities|Map|ForEachLoop(Map) (Utilities|Struct|BreakResourceAggregation ResourceAggregation))
    (:then
      (Development|PrintString (Utilities|String|Append (Utilities|String|EnumtoString (.stat _valuepin)) " 
Average: " (Utilities|String|ToString(Float) (.average _valuepin)) " 
Highest: " (Utilities|String|ToString(Text) (Variables|/Script/ProceduralCrafting.CraftingResource|GetName (.highest _valuepin))) " 
Influential: " (Utilities|String|ToString(Text) (Variables|/Script/ProceduralCrafting.CraftingResource|GetName (.mostinfluential _valuepin)))) true true "(R=0.000000,G=1.000000,B=0.051557,A=1.000000)" 99999999.0 (Utilities|String|StringToName (Utilities|String|EnumtoString (.stat _valuepin)))))))

(fn PrintWeaponStats
  (params (WeaponStats :type Weapon%20Stats%20Structure%20%28by%20ref%29) (WeaponType :type Weapon%20Type%20Object%20Reference%20%28by%20ref%29))
  (bind (_damage _durability _attackspeed) (Utilities|Struct|BreakWeaponStats WeaponStats))
  (bind _returnvalue (Utilities|GetObjectName WeaponType))
  (Development|PrintString (Utilities|String|Append _returnvalue " 
Damage: 
" (Utilities|String|ToString(Float) _damage) " 
Durability: 
" (Utilities|String|ToString(Float) _durability) " 
AttackSpeed: 
" (Utilities|String|ToString(Float) _attackspeed)) true true "(R=0.000000,G=1.000000,B=0.051269,A=1.000000)" 99999999.0 (Utilities|String|StringToName _returnvalue)))